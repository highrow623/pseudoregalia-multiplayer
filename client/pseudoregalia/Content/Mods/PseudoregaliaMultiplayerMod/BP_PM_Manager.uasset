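; Multiplayer mod manager for Pseudoregalia that displays other players as ghost actors in the local player's zone.
; Each Tick it packs the player's zone (level name) and location, passes them through SwapInfo, and feeds the result to UpdateGhosts.
; SwapInfo is an empty stub here.
; UpdateGhosts spawns, moves or destroys BP_PM_Ghost actors in an ID-keyed map by zone match, and removes ghosts whose IDs are absent.
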(event EventTick
  (params (DeltaSeconds :type Float%20%28single-precision%29))
  (bind _info (CallFunction|MakePlayerInfo))
  (bind _ghostinfo (CallFunction|SwapInfo _info))
  (CallFunction|UpdateGhosts _ghostinfo))

(event EventBeginPlay
  (bind _returnvalue (Game|GetCurrentLevelName true))
  (Variables|Default|SetZone _returnvalue)
  (bind _returnvalue_2 (Actor|GetActorOfClass "/Game/ThirdPerson/Player/BP_PlayerGoatMain.BP_PlayerGoatMain_C"))
  (Variables|Default|SetPlayerRef _returnvalue_2))

(fn ConstructionScript)

(fn MakePlayerInfo
  (return (Utilities|Struct|MakeF_PlayerInfo (Variables|Default|GetZone) (Transformation|GetActorLocation (Variables|Default|GetPlayerRef)))))

(fn SwapInfo
  (params (Info :type F%20Player%20Info%20Structure))
  (return 0))

(fn UpdateGhosts
  (params (GhostInfo :type Array%20of%20F%20Player%20Info%20Structures))
  (for _array_element GhostInfo
    (Utilities|Set|Add (LocalVariables|Getids) (Utilities|Struct|BreakF_PlayerInfo _array_element))
    (Utilities|DiagnoseInfo _array_element
      (:InZoneSpawned
        (CallFunction|UpdateGhost _array_element))
      (:InZoneNotSpawned
        (CallFunction|SpawnGhost _array_element))
      (:NotInZoneSpawned
        (CallFunction|RemoveGhost (Utilities|Struct|BreakF_PlayerInfo _array_element)))))
  (bind _keys (Utilities|Map|Keys (Variables|Default|GetGhosts)))
  (for _array_element_2 _keys
    (if (not (Utilities|Set|Contains (LocalVariables|Getids) _array_element_2))
      (CallFunction|RemoveGhost _array_element_2))))

(fn UpdateGhost
  (params (info :type F%20Player%20Info%20Structure))
  (bind (_id _location) (Utilities|Struct|BreakF_PlayerInfo info))
  (Transformation|SetActorLocation (.Value (Utilities|Map|Find (Variables|Default|GetGhosts) _id)) _location false false))

(fn SpawnGhost
  (params (info :type F%20Player%20Info%20Structure))
  (bind (_id _location) (Utilities|Struct|BreakF_PlayerInfo info))
  (bind _returnvalue (Game|SpawnActorfromClass "/Game/Mods/PseudoregaliaMultiplayerMod/BP_PM_Ghost.BP_PM_Ghost_C" (Math|Transform|MakeTransform _location "0, 0, 0" "1.000000,1.000000,1.000000") "AlwaysSpawn" 0 0))
  (Utilities|Map|Add (Variables|Default|GetGhosts) _id _returnvalue))

(fn RemoveGhost
  (params (id :type String))
  (bind _ghosts (Variables|Default|GetGhosts))
  (Utilities|FlowControl|Sequence
    (:then_0
      (Actor|DestroyActor (.Value (Utilities|Map|Find _ghosts id))))
    (:then_1
      (Utilities|Map|Remove _ghosts id))))