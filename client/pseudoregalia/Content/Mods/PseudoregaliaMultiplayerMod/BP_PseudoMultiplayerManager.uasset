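; Multiplayer mod manager for Pseudoregalia that shows players as BP_PseudoMultiplayerGhost actors in the current level.
; On BeginPlay it stores the level name as its Zone and keeps a map of spawned ghosts by Id.
; UpdateGhosts takes a list of ghost infos, and DiagnoseInfo routes each to spawn, move or remove by zone and spawn state.
; Ghosts missing from the list are destroyed, and updates set location only.
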(event EventTick
  (params (DeltaSeconds :type Float%20%28single-precision%29)))

(event EventBeginPlay
  (bind _returnvalue (Game|GetCurrentLevelName true))
  (Variables|Default|SetZone _returnvalue))

(fn ConstructionScript)

(fn UpdateGhosts
  (params (GhostInfo :type Array%20of%20Player%20Info%20Structures))
  (for _array_element GhostInfo
    (Utilities|Set|Add (LocalVariables|Getids) (Utilities|Struct|BreakPlayerInfo _array_element))
    (Utilities|DiagnoseInfo _array_element
      (:InZoneSpawned
        (CallFunction|UpdateGhost _array_element))
      (:InZoneNotSpawned
        (CallFunction|SpawnGhost _array_element))
      (:NotInZoneSpawned
        (CallFunction|RemoveGhost (Utilities|Struct|BreakPlayerInfo _array_element)))))
  (bind _keys (Utilities|Map|Keys (Variables|Default|GetGhosts)))
  (for _array_element_2 _keys
    (if (not (Utilities|Set|Contains (LocalVariables|Getids) _array_element_2))
      (CallFunction|RemoveGhost _array_element_2))))

(fn UpdateGhost
  (params (info :type Player%20Info%20Structure))
  (bind (_id _location) (Utilities|Struct|BreakPlayerInfo info))
  (Transformation|SetActorLocation (.Value (Utilities|Map|Find (Variables|Default|GetGhosts) _id)) _location false false))

(fn SpawnGhost
  (params (info :type Player%20Info%20Structure))
  (bind (_id _location) (Utilities|Struct|BreakPlayerInfo info))
  (bind _returnvalue (Game|SpawnActorfromClass "/Game/Mods/PseudoregaliaMultiplayerMod/BP_PseudoMultiplayerGhost.BP_PseudoMultiplayerGhost_C" (Math|Transform|MakeTransform _location "0, 0, 0" "1.000000,1.000000,1.000000") "AlwaysSpawn" 0 0))
  (Utilities|Map|Add (Variables|Default|GetGhosts) _id _returnvalue))

(fn RemoveGhost
  (params (id :type String))
  (bind _ghosts (Variables|Default|GetGhosts))
  (Utilities|FlowControl|Sequence
    (:then_0
      (Actor|DestroyActor (.Value (Utilities|Map|Find _ghosts id))))
    (:then_1
      (Utilities|Map|Remove _ghosts id))))