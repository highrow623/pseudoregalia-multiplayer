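; BP_PM_Ghost is a ghost actor in the Pseudoregalia multiplayer mod, with a SybilMesh component, that moves by simple extrapolation.
; Each Tick it adds Accel to Velocity, then teleports by Velocity, both scaled by delta time; nothing here sets Accel.
; An unconnected snippet, noted as usable on non-spirit-form meshes, would tint SybilMesh blue through the DieColor and DieAmount material parameters.
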(event EventTick
  (params (DeltaSeconds :type Float%20%28single-precision%29))
  (bind _returnvalue (Transformation|GetActorLocation))
  (bind _accel (Variables|Default|GetAccel))
  (bind _output_get (Variables|Default|SetVelocity (Math|Vector|MakeVector (+ (.x (Variables|Default|GetVelocity)) (* DeltaSeconds (.x _accel))) (+ (.y (Variables|Default|GetVelocity)) (* DeltaSeconds (.y _accel))) (+ (.z (Variables|Default|GetVelocity)) (* DeltaSeconds (.z _accel))))))
  (Transformation|SetActorLocation (Math|Vector|MakeVector (+ (* DeltaSeconds (.x _output_get)) (.x _returnvalue)) (+ (* DeltaSeconds (.y _output_get)) (.y _returnvalue)) (+ (* DeltaSeconds (.z _output_get)) (.z _returnvalue))) false true))

(event EventBeginPlay)

(fn ConstructionScript)